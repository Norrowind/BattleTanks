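; AutoMortar_BP is an automated mortar emplacement with an aiming component and a health bar widget.
; On BeginPlay it initializes TankAiming0 with the MortarDome as turret and MortarBarrel as barrel.
; It then hands itself to the HealthBar widget through the widget's TankBP reference, reusing tank aiming and health UI for the mortar.
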(event `self.ReceiveBeginPlay`
  (`TankAimingComponent.Initialize` (`self.TankAiming_0`) (`self.MortarDome`) (`self.MortarBarrel`))
  (`self.InitializeHealthBarWidget`))

(fn `InitializeHealthBarWidget`
  (bind _ashealth_bar (cast `/Game/UI/HealthBar` (`WidgetComponent.GetUserWidgetObject` (`self.HealthBar`))))
  (set `/Game/UI/HealthBar.Tank_BP` self _ashealth_bar))

(fn `UserConstructionScript`)